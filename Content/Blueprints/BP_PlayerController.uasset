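; Player controller that turns Enhanced Input actions into jump, look and movement for the BP_Player character.
; BeginPlay casts player character 0 to BP_Player and caches it, and each input event forwards to that reference without a validity check.
; Look feeds controller yaw and pitch, while Move applies movement along the character's own right and forward vectors rather than the control rotation.
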(event Input|EnhancedActionEvents|EnhancedInputActionIA_Jump
  (params (ActionValue :type Boolean) (ElapsedSeconds :type Float%20%28double-precision%29) (TriggeredSeconds :type Float%20%28double-precision%29) (InputAction :type Input%20Action%20Object%20Reference :default "/Game/Input/IA_Jump.IA_Jump"))
  (Character|Jump (Variables|Default|GetMyPlayer)))

(event Input|EnhancedActionEvents|EnhancedInputActionIA_Look
  (params (ActionValue :type Vector%202D%20Structure) (ElapsedSeconds :type Float%20%28double-precision%29) (TriggeredSeconds :type Float%20%28double-precision%29) (InputAction :type Input%20Action%20Object%20Reference :default "/Game/Input/IA_Look.IA_Look"))
  (bind _myplayer (Variables|Default|GetMyPlayer))
  (Pawn|Input|AddControllerYawInput _myplayer (.x ActionValue))
  (Pawn|Input|AddControllerPitchInput _myplayer (.y ActionValue)))

(event Input|EnhancedActionEvents|EnhancedInputActionIA_Move
  (params (ActionValue :type Vector%202D%20Structure) (ElapsedSeconds :type Float%20%28double-precision%29) (TriggeredSeconds :type Float%20%28double-precision%29) (InputAction :type Input%20Action%20Object%20Reference :default "/Game/Input/IA_Move.IA_Move"))
  (bind _myplayer (Variables|Default|GetMyPlayer))
  (Pawn|Input|AddMovementInput _myplayer (Transformation|GetActorRightVector _myplayer) (.x ActionValue) false)
  (Pawn|Input|AddMovementInput _myplayer (Transformation|GetActorForwardVector _myplayer) (.y ActionValue) false))

(event EventBeginPlay
  (bind _asbp_player (Utilities|Casting|CastToBP_Player (Game|GetPlayerCharacter 0)))
  (Variables|Default|SetMyPlayer _asbp_player) ; ddd
)

(event EventTick
  (params (DeltaSeconds :type Float%20%28single-precision%29)))

(fn ConstructionScript)